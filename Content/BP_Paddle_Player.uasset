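; Player-controlled paddle Blueprint that moves vertically along Z from the Move input axis.
; Each Tick it offsets its location by MoveSpeed times the axis value, blocking only movement further past hard-coded top and bottom bounds.
; The truncated axis value is stored in MoveDir, intended to help control the ball after it strikes the paddle.
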(event `self.ReceiveTick`
  (params (DeltaSeconds :type "Float (single-precision)"))
  (bind _returnvalue (`self.GetInputAxisValue`))
  (bind _z (.z (`self.K2_GetActorLocation`)))
  ;[1 1 1] Check if hitting the wall based on current position of Paddle
  (if (>= _z 1300.0)
    ;[1 1 1] If hitting top boundary, only adjust paddle if move input is downward
    (if (< (`self.GetInputAxisValue`) 0.0)
      ;[1 1 1] Paddle Movement, which will also help control ball after striking Paddle
      (`self.K2_AddActorLocalOffset` (`KismetMathLibrary.MakeVector` 0.0 0.0 (* (`self.moveSpeed`) _returnvalue)) :!label _label)
      (set `self.moveDir` (`KismetMathLibrary.FTrunc` _returnvalue)))
    (elif (<= _z 150.0)
      ;[1 1 1] If hitting bottom boundary, only adjust paddle if move input is upward
      (if (> (`self.GetInputAxisValue`) 0.0)
        (goto _label))
      (else
        (goto _label)))))

(fn `UserConstructionScript`)