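; Enemy paddle actor that moves vertically on its own to track the ball, as the AI opponent in a paddle-and-ball game.
; Each Tick it targets BP_Ball_Invisible if one exists, otherwise BP_Ball.
; SetDirection compares heights, with a small dead zone, to choose up, down or still.
; It then applies a fixed per-frame Z offset, not scaled by delta time, blocking movement past the top and bottom limits.
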(event `self.ReceiveTick`
  (params (DeltaSeconds :type "Float (single-precision)"))
  (bind _z (.z (`self.K2_GetActorLocation`)))
  ;[1 1 1] check if it exists and use it as reference, otherwise use regular ball
  (bind _returnvalue (`GameplayStatics.GetActorOfClass` "/Game/BP_Ball_Invisible.BP_Ball_Invisible_C"))
  (if (`KismetSystemLibrary.IsValid` _returnvalue)
    (set `self.tarPositionEnemy` (`self.K2_GetActorLocation` _returnvalue))
    (else
      ;[1 1 1] Enemy Paddle Movement AI
      (bind _returnvalue_2 (`GameplayStatics.GetActorOfClass` "/Game/BP_Ball.BP_Ball_C"))
      (set `self.tarPositionEnemy` (`self.K2_GetActorLocation` _returnvalue_2))))
  ;;[1 1 1] Custom Function
  (`self.SetDirection`)
  ;[1 1 1] Check if paddle location is within bounds before moving (adding offset)
  (if (>= _z 1300.0)
    ;[1 1 1] If hitting top boundary, only adjust paddle if move input is downward
    (if (== (`self.moveDirEnemy`) -1)
      (`self.K2_AddActorLocalOffset` (`KismetMathLibrary.MakeVector` 0.0 0.0 (* (`self.moveDirEnemy`) (`self.moveSpeedEnemy`))) :!label _label))
    (elif (<= _z 150.0)
      ;[1 1 1] If hitting bottom boundary, only adjust paddle if move input is upward
      (if (== (`self.moveDirEnemy`) 1)
        (goto _label))
      (else
        (goto _label)))))

(fn `SetDirection`
  ;[1 1 1] Is the ball above enemy, even with enemy, or below enemy?
  ;[1 1 1] check if paddle is location is less than (lower) than target (ball)
  (if (>= (`KismetMathLibrary.Abs` (- (.z (`self.K2_GetActorLocation`)) (.z (`self.tarPositionEnemy`)))) 10.0)
    ;[1 1 1] set paddle movement updwards
    (if (<= (.z (`self.K2_GetActorLocation`)) (.z (`self.tarPositionEnemy`)))
      (bind _output_get (set `self.moveDirEnemy` 1))
      (elif (>= (.z (`self.K2_GetActorLocation`)) (.z (`self.tarPositionEnemy`)))
        ;[1 1 1] set paddle movement downwards
        (bind _output_get_2 (set `self.moveDirEnemy` -1))
        (else
          ;[1 1 1] no movement direction
          (bind _output_get_3 (set `self.moveDirEnemy` 0 :!label _label)))))
    (else
      (goto _label))))

(fn `UserConstructionScript`)