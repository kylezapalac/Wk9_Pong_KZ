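; Pong-style ball that moves by projectile movement, bouncing between player and enemy paddles and off walls.
; Paddle overlaps reverse X, add random spin biased by paddle direction, compound speed using a bounce count, and spawn an invisible ball with doubled horizontal velocity.
; Walls reverse Z, with a short shared cooldown guarding both reversals.
; Tick resets position, velocity and bounce count once the ball passes either paddle.
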(event `self.ReceiveActorBeginOverlap`
  (params (OtherActor :type "Actor Object Reference"))
  ;[1 1 1] Update travel direction of ball based on contact with the paddles or with the wall
  (bind _asbp_paddle_player (cast `/Game/BP_Paddle_Player` OtherActor)
    (:`then`
      (`self.HandleBounce` (`/Game/BP_Paddle_Player.moveDir` _asbp_paddle_player))
      ;[1 1 1] I created invisible ball in here?
      (bind _returnvalue (`|SpawnActorFromClass` "/Game/BP_Ball_Invisible.BP_Ball_Invisible_C" (`self.GetTransform`) "Undefined" "OverrideRootScale" null null :!label _label))
      (if (`KismetSystemLibrary.IsValid` _returnvalue)
        (bind _projectilemovement (`/Game/BP_Ball_Invisible.ProjectileMovement` _returnvalue))
        (set `MovementComponent.Velocity` (`KismetMathLibrary.MakeVector` (* (.x (`MovementComponent.Velocity` _projectilemovement)) 2.0)) _projectilemovement)))
    (:`CastFailed`
      (bind _asbp_paddle_enemy (cast `/Game/BP_Paddle_Enemy` OtherActor)
        (:`then`
          (`self.HandleBounce` (`/Game/BP_Paddle_Enemy.moveDirEnemy` _asbp_paddle_enemy))
          (goto _label))
        (:`CastFailed`
          (cast `/Game/BP_Wall` OtherActor)
          (`self.ReverseZ`))))))

(event `self.ReceiveTick`
  (params (DeltaSeconds :type "Float (single-precision)"))
  ;[1 1 1] When ball goes out of bounds, reset location to intial position and apply last velocity. Also reset bounce count to 0, so that we can reset speed of ball to default.
  (set `self.TimeSinceReversed` (+ DeltaSeconds (`self.TimeSinceReversed`)))
  (bind _outofbounds (`self.IsOutOfBounds`))
  (if _outofbounds
    (set `self.BounceCount` 0.0)
    (`self.K2_SetActorLocation` (0.0 90.0 770.0))
    (set `MovementComponent.Velocity` (`KismetMathLibrary.MakeVector` -300.0) (`self.ProjectileMovement`))))

(fn `AddSpeed`
  (bind _projectilemovement (`self.ProjectileMovement`))
  ;[1 1 1] Get current bounce count and increment by 1
  (bind _output_get (set `self.BounceCount` (+ (`self.BounceCount`) 1.0)))
  (set `MovementComponent.Velocity` (`KismetMathLibrary.MakeVector` (* (.x (`MovementComponent.Velocity` _projectilemovement)) (+ (/ _output_get 50.0) 1.0)) (.y (`MovementComponent.Velocity` _projectilemovement)) (.z (`MovementComponent.Velocity` _projectilemovement))) _projectilemovement))

(fn `AddSpin`
  (params (Spin :type "Float (double-precision)"))
  (bind _projectilemovement (`self.ProjectileMovement`))
  ;[1 1 1] Set velocity (up or down slightly)
  (set `MovementComponent.Velocity` (+ (`KismetMathLibrary.MakeVector` 0.0 0.0 Spin) (`MovementComponent.Velocity` _projectilemovement)) _projectilemovement))

(fn `HandleBounce`
  (params (Selection :type Integer))
  (bind _returnvalue (`KismetMathLibrary.RandomFloatInRange` -50.0 50.0))
  (switch `int` Selection
    (:`-1`
      (`self.AddSpin` (+ _returnvalue -125.0)))
    (:`0`
      (`self.AddSpin` (`KismetMathLibrary.RandomFloatInRange` -15.0 15.0)))
    (:`1`
      (`self.AddSpin` (+ _returnvalue 125.0))))
  (`self.ReverseX`)
  (`self.AddSpeed`))

(fn `IsOutOfBounds`
  (returns (OutOfBounds :type Boolean))
  ;[1 1 1] Checking if ball has gone past player paddle, else if past enemy paddle
  ;[1 1 1] Past Player Paddle?
  (bind _outactors (`GameplayStatics.GetAllActorsOfClass` "/Game/BP_Paddle_Player.BP_Paddle_Player_C"))
  (if (not (<= (.x (`self.K2_GetActorLocation`)) (- (.x (`self.K2_GetActorLocation` (`|GetArrayItem` _outactors))) 150.0)))
    ;[1 1 1] Past Enemy Paddle?
    (bind _outactors_2 (`GameplayStatics.GetAllActorsOfClass` "/Game/BP_Paddle_Enemy.BP_Paddle_Enemy_C"))
    (if (>= (.x (`self.K2_GetActorLocation`)) (+ (.x (`self.K2_GetActorLocation` (`|GetArrayItem` _outactors_2))) 150.0))
      _
      (else
        (return false))))
  (return true))

(fn `ReverseX`
  (bind _projectilemovement (`self.ProjectileMovement`))
  (if (>= (`self.TimeSinceReversed`) 0.01)
    (set `MovementComponent.Velocity` (`KismetMathLibrary.MakeVector` (* (.x (`MovementComponent.Velocity` _projectilemovement)) -1.0) (.y (`MovementComponent.Velocity` _projectilemovement)) (.z (`MovementComponent.Velocity` _projectilemovement))) _projectilemovement)
    (`KismetSystemLibrary.PrintString` "REVERSE X")
    (set `self.TimeSinceReversed` 0.0)))

(fn `ReverseZ`
  (bind _projectilemovement (`self.ProjectileMovement`))
  (if (>= (`self.TimeSinceReversed`) 0.01)
    (set `MovementComponent.Velocity` (`KismetMathLibrary.MakeVector` (.x (`MovementComponent.Velocity` _projectilemovement)) (.y (`MovementComponent.Velocity` _projectilemovement)) (* (.z (`MovementComponent.Velocity` _projectilemovement)) -1.0)) _projectilemovement)
    (`KismetSystemLibrary.PrintString` "REVERSE Z")
    (set `self.TimeSinceReversed` 0.0)))

(fn `UserConstructionScript`)